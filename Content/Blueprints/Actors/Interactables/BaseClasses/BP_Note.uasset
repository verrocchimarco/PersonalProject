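; BP_Note is an interactable note actor that the game records as found when something interacts with it.
; On DoInteract it runs the parent behavior, then passes its NoteIndex to SetNoteAsFound on BP_InnerSanctumGameInstance and destroys itself.
; The found state is handed to the game instance rather than kept on the actor, and the note has no active BeginPlay, overlap or Tick logic.
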(event `InteractInterface.DoInteract`
  (params (InteractingActor :type "Actor Object Reference"))
  (`parent.DoInteract` InteractingActor)
  (`InnerSanctumGameInstance.SetNoteAsFound` (cast `/Game/Blueprints/GameSystem/BP_InnerSanctumGameInstance` (`GameplayStatics.GetGameInstance`) :!pure true) (`self.NoteIndex`))
  (`self.K2_DestroyActor`))

(fn `UserConstructionScript`
  (`parent.UserConstructionScript`))