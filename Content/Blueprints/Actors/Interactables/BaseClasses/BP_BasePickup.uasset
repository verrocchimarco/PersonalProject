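; Base interactable pickup that grants an assigned item actor to the protagonist's inventory when interacted with.
; On BeginPlay it spawns the assigned class at its own transform as a hidden, non-colliding actor.
; Interaction adds that actor to the inventory component, attaches it to the player and destroys the pickup.
; A failed add briefly tints the emissive material with a reject color, then resets it to white.
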(event `self.ReceiveBeginPlay`
  (`parent.ReceiveBeginPlay`)
  (set `self.Protagonist Character Ref` (cast `/Game/Blueprints/Characters/BP_ProtagonistCharacter` (`GameplayStatics.GetPlayerPawn` 0) :!pure true))
  (bind _returnvalue (`|SpawnActorFromClass` (`self.Assigned Object`) (`self.GetTransform`) "AlwaysSpawn" "OverrideRootScale" null null))
  (bind _output_get (set `self.Spawned Object` _returnvalue))
  (`self.SetActorHiddenInGame` _output_get true)
  (`self.SetActorEnableCollision` _output_get false))

(event `InteractInterface.DoInteract`
  (params (InteractingActor :type "Actor Object Reference"))
  (`parent.DoInteract` InteractingActor)
  (bind _returnvalue (`InventoryComponent.AddItem` (`ProtagonistCharacter.uInventoryComponent` (`self.Protagonist Character Ref`)) (`self.Spawned Object`)))
  (if _returnvalue
    (`self.K2_AttachToActor` (`self.Spawned Object`) (`self.Protagonist Character Ref`) "None" "SnapToTarget" "KeepRelative" "KeepRelative" false)
    (`self.K2_DestroyActor`)
    (else
      (`MaterialInstanceDynamic.SetVectorParameterValue` (`self.DynamicEmissiveMaterial`) "EmissiveColor" (`self.Pickup Reject Color`))
      (`KismetSystemLibrary.Delay` 1.2)
      (`MaterialInstanceDynamic.SetVectorParameterValue` (`self.DynamicEmissiveMaterial`) "EmissiveColor" (struct :`R` 1.0 :`G` 1.0 :`B` 1.0 :`A` 1.0)))))

(fn `UserConstructionScript`
  (`parent.UserConstructionScript`))