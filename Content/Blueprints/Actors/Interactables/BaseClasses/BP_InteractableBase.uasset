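; Base interactable actor that supplies a glow highlight, a button prompt and an interaction hook.
; The construction script creates a dynamic instance of the emissive mesh's material, which SetVisibilityGlow drives through scalar parameters, switching the glow off after a short delay.
; GetPromptDescription prefixes the prompt text with the Space or E key label from the configured button response, also returned by GetInteractionType.
; DoInteract simply forwards the interacting actor to ParentDoInteract.
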(event `InteractInterface.SetVisibilityGlow`
  (bind _dynamicemissivematerial (`self.DynamicEmissiveMaterial`))
  (bind _dynamicemissivematerial_2 (`self.DynamicEmissiveMaterial`))
  (if (not (`self.bShouldGlow`))
    (set `self.bShouldGlow` true)
    (`MaterialInstanceDynamic.SetScalarParameterValue` _dynamicemissivematerial_2 "EmissiveMaxStrength" (`self.EmissiveMaterialMaxStrength`))
    (`MaterialInstanceDynamic.SetScalarParameterValue` _dynamicemissivematerial_2 "EmissiveDeltaTime" (`self.EmissiveMaterialDeltaTime`))
    (set `self.bShouldGlow` false)
    (`KismetSystemLibrary.Delay` 1.5)
    (if (not (`self.bShouldGlow`))
      (`MaterialInstanceDynamic.SetScalarParameterValue` _dynamicemissivematerial "EmissiveMaxStrength" 0.0)
      (`MaterialInstanceDynamic.SetScalarParameterValue` _dynamicemissivematerial "EmissiveDeltaTime" 0.0))))

(event `InteractInterface.DoInteract`
  (params (InteractingActor :type "Actor Object Reference"))
  (`parent.DoInteract` InteractingActor))

(fn `GetInteractionType`
  (returns (ReturnValue :type "InteractionType Enum"))
  (return (`self.InteractableButtonResponse`)))

(fn `GetPromptDescription`
  (returns (ReturnValue :type Text))
  (return (`KismetTextLibrary.Conv_StringToText` (`KismetStringLibrary.Concat_StrStr` (`KismetTextLibrary.Conv_TextToString` (select `InteractionType` (`self.InteractableButtonResponse`) :`SpaceButton` "[Space] " :`EButton` "[E] ")) (`KismetTextLibrary.Conv_TextToString` (`self.PromptDescription`))))))

(fn `UserConstructionScript`
  (bind _emissivemesh (`self.EmissiveMesh`))
  (bind _emissivematerialindex (`self.EmissiveMaterialIndex`))
  (bind _returnvalue (`PrimitiveComponent.CreateDynamicMaterialInstance` _emissivemesh _emissivematerialindex (`PrimitiveComponent.GetMaterial` _emissivemesh _emissivematerialindex) "None"))
  (set `self.DynamicEmissiveMaterial` _returnvalue))