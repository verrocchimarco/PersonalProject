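; Interactable door that a character swings open or closed, toggling its "Open"/"Close" prompt when the swing finishes.
; On interaction, the RotateDoor timeline plays or reverses to drive the door's yaw, at a faster slam rate for running openers.
; Swing direction is the rounded dot product of door and interactor facing (camera for the protagonist), retained for closing.
; The Space interaction is only a placeholder print.
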(event `self.ReceiveBeginPlay`
  (`parent.ReceiveBeginPlay`))

(event `ChangePromptOnInteract`
  (bind _output_get (set `self.isOpen` (not (`self.isOpen`))))
  (if _output_get
    (set `self.PromptDescriptionE` "Close")
    (else
      (set `self.PromptDescriptionE` "Open"))))

(event `InteractInterface.DoInteract`
  (params (InteractingActor :type "Actor Object Reference") (ButtonPressed :type "InteractionType Enum" :default "SpaceButton"))
  (`parent.DoInteract` InteractingActor ButtonPressed))

(event `self.InteractionE`
  (params (InteractingActor :type "Actor Object Reference"))
  (bind _asbase_character (cast `BaseCharacter` InteractingActor))
  (`self.ComputeOpeningFunction` _asbase_character)
  (if (`self.isOpen`)
    (bind (_direction _rotation) (`Timeline|RotateDoor` :!via `Reverse` :!label _label)
      (:`Update`
        (`SceneComponent.K2_SetRelativeRotation` (`self.Door`) (`KismetMathLibrary.MakeRotator` 0.0 0.0 (* (`self.DotProduct`) _rotation)) false false))
      (:`Finished`
        (`self.ChangePromptOnInteract`)))
    (else
      (goto _label))))

(event `self.InteractionSpace`
  (params (InteractingActor :type "Actor Object Reference"))
  (`KismetSystemLibrary.PrintString` "Some Day..."))

(fn `ComputeOpeningFunction`
  (params (InteractingActor :type "BaseCharacter Object Reference"))
  (locals (Actor :type "BaseCharacter Object Reference") (ActorForwardVector :type "Vector Structure"))
  ;[1 1 1] Compute Dot Vector based on either camera for player or rotation for enemies
  (bind _output_get (set `local.Actor` InteractingActor))
  (bind _asprotagonist_character (cast `ProtagonistCharacter` _output_get)
    (:`then`
      (set `local.ActorForwardVector` (`SceneComponent.GetForwardVector` (`ProtagonistCharacter.GetCamera` _asprotagonist_character))))
    (:`CastFailed`
      (set `local.ActorForwardVector` (`KismetMathLibrary.GetForwardVector` (`self.K2_GetActorRotation` (`local.Actor`))))))
  ;[1 1 1] Only compute Dot Vector if the door needs to be opened. Else keep old Dot Value for reversal (door close)
  (if (not (`self.isOpen`))
    (set `self.DotProduct` (`KismetMathLibrary.Conv_IntToDouble` (`KismetMathLibrary.Round` (`KismetMathLibrary.Dot_VectorVector` (`self.GetActorForwardVector` self) (`local.ActorForwardVector`))))))
  (if (and (`BaseCharacter.GetIsRunning` (`local.Actor`)) (not (`self.isOpen`)))
    (set `self.RotationTime` (`self.SlamOpenTime`))
    (else
      (set `self.RotationTime` (`self.NormalOpenTime`))))
  (`TimelineComponent.SetPlayRate` (`self.RotateDoor`) (/ 1.0 (`self.RotationTime`))))

(fn `UserConstructionScript`
  (`parent.UserConstructionScript`))