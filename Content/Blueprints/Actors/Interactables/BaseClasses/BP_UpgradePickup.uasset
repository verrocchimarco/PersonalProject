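; Base interactable pickup that grants the player an upgrade when interacted with.
; On BeginPlay it caches the protagonist character.
; DoInteract constructs an object from the AssociatedUpgrade class, assigns it the protagonist and passes it to the inventory component's AddUpgrade.
; The result routes to AddUpgradeSuccess or AddUpgradeFailure, both empty events in this class.
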(event `self.ReceiveBeginPlay`
  (`parent.ReceiveBeginPlay`)
  (set `self.Protagonist Character Ref` (cast `/Game/Blueprints/Characters/BP_ProtagonistCharacter` (`GameplayStatics.GetPlayerPawn` 0) :!pure true)))

(event `self.DoInteract`
  (params (InteractingActor :type "Actor Object Reference"))
  (bind _protagonist_character_ref (`self.Protagonist Character Ref`))
  (`parent.DoInteract` InteractingActor)
  ;[1 1 1] Add upgrade component to pickup actor
  (bind _returnvalue (`|GenericCreateObject` (`self.Associated Upgrade`)))
  (`Upgrade.SetMainCharacter` _returnvalue _protagonist_character_ref)
  ;[1 1 1] Call component's "add upgrade"
  (bind _returnvalue_2 (`InventoryComponent.AddUpgrade` (`ProtagonistCharacter.uInventoryComponent` _protagonist_character_ref) _returnvalue))
  (if _returnvalue_2
    (`self.AddUpgrade Success`)
    (else
      (`self.AddUpgrade Failure`))))

(event `AddUpgrade Failure`)

(event `AddUpgrade Success`)

(fn `UserConstructionScript`
  (`parent.UserConstructionScript`))