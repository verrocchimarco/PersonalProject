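; BP_LostBackpack is a physics-simulated interactable pickup that gives the player a backpack.
; On interact, it passes its emissive mesh's static mesh to the protagonist's inventory component as the backpack mesh, then enables the backpack.
; A looping one-second timer polls that inventory, so the actor destroys itself once the player has any backpack, whether from this pickup or another.
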(event `self.ReceiveBeginPlay`
  (`parent.ReceiveBeginPlay`)
  (set `self.Inventory Component` (`ProtagonistCharacter.uInventoryComponent` (cast `/Game/Blueprints/Characters/BP_ProtagonistCharacter` (`GameplayStatics.GetPlayerPawn` 0) :!pure true)))
  (`PrimitiveComponent.SetSimulatePhysics` (`self.EmissiveMesh`) true)
  ;[1 1 1] Check every X seconds if the player has found a backpack (self or another one). Destroy actor if a backpack is found
  (bind _returnvalue (`KismetSystemLibrary.K2_SetTimerDelegate` (delegate `PlayerHasFoundBackpack`) 1.0 true)))

(event `PlayerHasFoundBackpack`
  ;[1 1 1] Check every X seconds if the player has found a backpack (self or another one). Destroy actor if a backpack is found
  (if (`InventoryComponent.hasBackpack` (`self.Inventory Component`))
    (`KismetSystemLibrary.K2_ClearAndInvalidateTimerHandle` (stale `self.ReceiveBeginPlay` _returnvalue))
    (`self.K2_DestroyActor`)))

(event `InteractInterface.DoInteract`
  (params (InteractingActor :type "Actor Object Reference"))
  (bind _inventory_component (`self.Inventory Component`))
  (`parent.DoInteract` InteractingActor)
  (`InventoryComponent.SetBackpackMesh` _inventory_component (`StaticMeshComponent.StaticMesh` (`self.EmissiveMesh`)))
  (`InventoryComponent.EnableBackpack` _inventory_component)
  (`self.PlayerHasFoundBackpack`))

(fn `UserConstructionScript`
  (`parent.UserConstructionScript`))