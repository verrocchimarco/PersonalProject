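; BP_InteractableBase is a base actor for interactable objects, exposing a prompt description and an interaction type.
; Its construction script creates a dynamic material instance on the emissive mesh's designated slot.
; SetVisibilityGlow and UnsetVisibilityGlow drive that material's emissive strength and time parameters to switch the highlight on and off.
; DoInteract is only a placeholder that prints a debug string.
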(event `InteractInterface.SetVisibilityGlow`
  (bind _interactionmaterial (`self.InteractionMaterial`))
  (`MaterialInstanceDynamic.SetScalarParameterValue` _interactionmaterial "EmissiveMaxStrength" (`self.EmissiveMaterialMaxStrength`))
  (`MaterialInstanceDynamic.SetScalarParameterValue` _interactionmaterial "EmissiveDeltaTime" (`self.EmissiveMaterialDeltaTime`)))

(event `InteractInterface.UnsetVisibilityGlow`
  (bind _interactionmaterial (`self.InteractionMaterial`))
  (`MaterialInstanceDynamic.SetScalarParameterValue` _interactionmaterial "EmissiveMaxStrength" 0.0)
  (`MaterialInstanceDynamic.SetScalarParameterValue` _interactionmaterial "EmissiveDeltaTime" 0.0))

(event `InteractInterface.DoInteract`
  (params (InteractingActor :type "Actor Object Reference"))
  (`KismetSystemLibrary.PrintString` "Uhhh you touched my lalala"))

(fn `GetInteractionType`
  (returns (ReturnValue :type "InteractionType Enum"))
  (return (`self.InteractionType`)))

(fn `GetPromptDescription`
  (returns (ReturnValue :type Text))
  (return (`KismetTextLibrary.Conv_StringToText` (`self.PromptDescription`))))

(fn `UserConstructionScript`
  (bind _returnvalue (`self.GetEmissiveMaterialIndex`))
  (bind _emissivemesh (`self.EmissiveMesh`))
  (bind _returnvalue_2 (`PrimitiveComponent.CreateDynamicMaterialInstance` _emissivemesh _returnvalue (`PrimitiveComponent.GetMaterial` _emissivemesh _returnvalue) "None"))
  (set `self.InteractionMaterial` _returnvalue_2))