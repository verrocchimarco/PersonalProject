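; BP_InteractableBase is a base actor for world interactables that can glow, show a prompt and be interacted with.
; Its construction script creates a dynamic material instance on a chosen slot of EmissiveMesh, and the glow events set or zero its emissive strength and delta-time parameters.
; Getters expose the prompt description and movement displacement type, while DoInteract only prints a placeholder debug string.
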(event `InteractInterface.SetVisibilityGlow`
  (bind _dynamicemissivematerial (`self.DynamicEmissiveMaterial`))
  (`MaterialInstanceDynamic.SetScalarParameterValue` _dynamicemissivematerial "EmissiveMaxStrength" (`self.EmissiveMaterialMaxStrength`))
  (`MaterialInstanceDynamic.SetScalarParameterValue` _dynamicemissivematerial "EmissiveDeltaTime" (`self.EmissiveMaterialDeltaTime`)))

(event `InteractInterface.UnsetVisibilityGlow`
  (bind _dynamicemissivematerial (`self.DynamicEmissiveMaterial`))
  (`MaterialInstanceDynamic.SetScalarParameterValue` _dynamicemissivematerial "EmissiveMaxStrength" 0.0)
  (`MaterialInstanceDynamic.SetScalarParameterValue` _dynamicemissivematerial "EmissiveDeltaTime" 0.0))

(event `InteractInterface.DoInteract`
  (params (InteractingActor :type "Actor Object Reference"))
  (`KismetSystemLibrary.PrintString` "Uhhh you touched my lalala"))

(fn `GetInteractionType`
  (returns (ReturnValue :type "InteractionType Enum"))
  (return (`self.InteractableMovementDisplacement`)))

(fn `GetPromptDescription`
  (returns (ReturnValue :type Text))
  (return (`self.PromptDescription`)))

(fn `UserConstructionScript`
  (bind _emissivemesh (`self.EmissiveMesh`))
  (bind _emissivematerialindex (`self.EmissiveMaterialIndex`))
  (bind _returnvalue (`PrimitiveComponent.CreateDynamicMaterialInstance` _emissivemesh _emissivematerialindex (`PrimitiveComponent.GetMaterial` _emissivemesh _emissivematerialindex) "None"))
  (set `self.DynamicEmissiveMaterial` _returnvalue))