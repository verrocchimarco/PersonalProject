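; Medium backpack upgrade pickup that unlocks the backpack for the player's inventory.
; It overrides the parent's AddUpgradeSuccess event, runs the parent logic, then calls EnableBackpack on the protagonist character's inventory component.
; The pickup destroys itself afterwards, and all other events are left to the parent.
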(event `self.AddUpgrade Success`
  (`parent.AddUpgrade Success`)
  (`InventoryComponent.EnableBackpack` (`ProtagonistCharacter.uInventoryComponent` (cast `/Game/Blueprints/Characters/BP_ProtagonistCharacter` (`GameplayStatics.GetPlayerPawn` 0) :!pure true)))
  (`self.K2_DestroyActor`))

(fn `UserConstructionScript`
  (`parent.UserConstructionScript`))