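; Base pickup interactable that adds an item of its AssignedObject class to the protagonist's inventory.
; On BeginPlay it caches the player character and the controller's inventory widget, though the widget is unused here.
; On DoInteract it spawns the item hidden at its own transform and passes it to the inventory component's AddItem.
; The pickup destroys itself only if the add succeeds; a failed add leaves the hidden spawned actor in place.
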(event `self.ReceiveBeginPlay`
  (`parent.ReceiveBeginPlay`)
  (set `self.Protagonist Character Ref` (cast `/Game/Blueprints/Characters/BP_ProtagonistCharacter` (`GameplayStatics.GetPlayerPawn` 0) :!pure true))
  (set `self.Character Widget Inventory` (`ProtagonistController.WidgetInventory` (cast `/Game/Blueprints/GameSystem/BP_ProtagonistController` (`GameplayStatics.GetPlayerController` 0) :!pure true))))

(event `InteractInterface.DoInteract`
  (params (InteractingActor :type "Actor Object Reference"))
  (`parent.DoInteract` InteractingActor)
  (bind _returnvalue (`|SpawnActorFromClass` (`self.Assigned Object`) (`self.GetTransform`) "Undefined" "OverrideRootScale" null null))
  (`self.SetActorHiddenInGame` _returnvalue true)
  (bind _returnvalue_2 (`InventoryComponent.AddItem` (`ProtagonistCharacter.uInventoryComponent` (`self.Protagonist Character Ref`)) _returnvalue))
  (if _returnvalue_2
    (`self.K2_DestroyActor`)))

(fn `UserConstructionScript`
  (`parent.UserConstructionScript`))