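; BP_ProtagonistCharacter is the protagonist character Blueprint, extending interaction prompt behavior from its parent.
; The UpdateInteractionWidget override calls the parent, then passes the interactable actor's prompt description to the W_InteractPrompt widget held by a widget component.
; Debug keys print the health component's current health and apply point damage to the character itself.
; BeginPlay, Tick, overlap and the construction script contain no logic.
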(event `self.ReceiveBeginPlay`)

(event `self.UpdateInteractionWidget`
  (params (InteractableActor :type "Actor Object Reference") (TraceImpactPoint :type "Vector Structure"))
  (`parent.UpdateInteractionWidget` InteractableActor TraceImpactPoint)
  (bind _returnvalue (message `InteractInterface.GetPromptDescription` InteractableActor))
  (`/Game/UMG/W_InteractPrompt.UpdatePromptDescription` (cast `/Game/UMG/W_InteractPrompt` (`WidgetComponent.GetUserWidgetObject` (`self.wInteractPrompt`)) :!pure true) _returnvalue))

(event `Key|Two`
  (params (Key :type "Key Structure"))
  (:`Pressed`
    (`KismetSystemLibrary.PrintString` (`KismetStringLibrary.Conv_DoubleToString` (`HealthComponent.GetCurrentHealth` (`self.uHealthComponent`))))))

(event `Key|Three`
  (params (Key :type "Key Structure"))
  (bind _returnvalue (`SceneComponent.K2_GetComponentLocation` (`self.Mesh`)))
  (:`Pressed`
    (`GameplayStatics.ApplyPointDamage` self 10.0 (`self.K2_GetActorLocation` self) (`GameplayStatics.MakeHitResult` false false 0.0 0.0 _returnvalue _returnvalue))))

(fn `UserConstructionScript`)